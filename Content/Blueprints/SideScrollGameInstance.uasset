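; Game instance for a side-scroller that holds stage-clear progress and manages the stage select screen.
; ShowStageSelectWidget lazily creates and caches the StageSelect widget, then adds it to or removes it from the viewport.
; Save copies ClearStage into a SideScrollSaveGameBP object, created if missing, and writes it to a fixed slot.
; Load reads that slot back, caches the save object and restores ClearStage, stopping if the cast fails.
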(fn `Load`
  (bind _returnvalue (`GameplayStatics.LoadGameFromSlot` "SideScroll"))
  (bind _asside_scroll_save_game_bp (cast `/Game/Blueprints/SideScrollSaveGameBP` _returnvalue))
  (bind _output_get (set `self.SideScrollSaveGameRef` _asside_scroll_save_game_bp))
  (set `self.ClearStage` (`/Game/Blueprints/SideScrollSaveGameBP.ClearStage` _output_get)))

(fn `Save`
  (bind _sidescrollsavegameref (`self.SideScrollSaveGameRef`))
  (`/Engine/EditorBlueprintResources/StandardMacros.IsValid` (`self.SideScrollSaveGameRef`)
    (:`Is Valid`
      _)
    (:`Is Not Valid`
      (bind _returnvalue (`GameplayStatics.CreateSaveGameObject` "/Game/Blueprints/SideScrollSaveGameBP.SideScrollSaveGameBP_C"))
      (set `self.SideScrollSaveGameRef` _returnvalue)))
  (set `/Game/Blueprints/SideScrollSaveGameBP.ClearStage` (`self.ClearStage`) _sidescrollsavegameref)
  (`GameplayStatics.SaveGameToSlot` _sidescrollsavegameref "SideScroll"))

(fn `ShowStageSelectWidget`
  (params (IsShow :type Boolean))
  (bind _stageselectui (`self.StageSelectUI`))
  (`/Engine/EditorBlueprintResources/StandardMacros.IsValid` (`self.StageSelectUI`)
    (:`Is Valid`
      _)
    (:`Is Not Valid`
      (bind _returnvalue (`|CreateWidget` "/Game/Blueprints/UI/StageSelect.StageSelect_C" (`GameplayStatics.GetPlayerController` 0)))
      (set `self.StageSelectUI` _returnvalue)))
  (if IsShow
    (`UserWidget.AddToViewport` _stageselectui 0)
    (else
      (`Widget.RemoveFromParent` _stageselectui))))