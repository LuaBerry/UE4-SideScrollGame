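; Goblin monster Character that chases and melees the player along the Y axis, with a floating HP bar and damage numbers.
; Tick refreshes player distance and direction and runs the idle, follow and attack states, halting on player death or stage clear.
; Animation-driven events toggle a hit capsule that damages tagged characters with a different actor tag.
; Cooldown-gated damage triggers particles, sound, material flash and knockback, then impact or delayed destruction on death.
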(event `self.ReceiveBeginPlay`
  (bind _returnvalue (`|SpawnActorFromClass` "/Game/Blueprints/Etc/CharHPBarBP.CharHPBarBP_C" (`KismetMathLibrary.Conv_VectorToTransform` (`SceneComponent.K2_GetComponentLocation` (`self.Cube_HPBarPosDummy`))) "Undefined" "OverrideRootScale" null null))
  (set `self.CharHPBarRef` _returnvalue))

(event `GetDistance_And_Direction`
  (bind _y (.y (- (`self.K2_GetActorLocation` (`GameplayStatics.GetPlayerCharacter` 0)) (`self.K2_GetActorLocation`))))
  (bind _asdefault_play_game_mode (cast `/Game/Blueprints/DefaultPlayGameMode` (`GameplayStatics.GetGameMode`)))
  (set `self.isStageClear` (`|EnumEquality` (`/Game/Blueprints/DefaultPlayGameMode.CurGameplayState` _asdefault_play_game_mode) "NewEnumerator2"))
  (bind _aspaladin_bp (cast `/Game/Blueprints/PaladinBP` (`GameplayStatics.GetPlayerCharacter` 0)))
  (set `self.isDeathPlayerChar` (`/Game/Blueprints/PaladinBP.isDeath` _aspaladin_bp))
  (set `self.DistancePlayerChar` (`KismetMathLibrary.Abs` _y))
  (set `self.DirToPlayerChar` (`KismetMathLibrary.Normal` (`KismetMathLibrary.MakeVector` 0.0 _y))))

(event `OnAnimEnd_Attack`
  (set `self.isAttacking` false)
  (set `self.CurState` "NewEnumerator2"))

(event `Attack`
  (set `self.isAttacking` true)
  (`self.K2_SetActorRotation` (`KismetMathLibrary.Conv_VectorToRotator` (`self.DirToPlayerChar`)))
  (`self.PlayAnimMontage` "/Game/Mesh/Goblin/Animations/AnimMontage/goblin_slash_Montage.goblin_slash_Montage"))

(event `OnAnimEnd_Impact`
  (set `self.isAttacking` false)
  (set `self.CurState` "NewEnumerator2"))

(event `self.ReceiveTick`
  (params (DeltaSeconds :type "Float (single-precision)"))
  (set `self.TimefromLastDamage` (+ DeltaSeconds (`self.TimefromLastDamage`)))
  (`self.GetDistance_And_Direction`)
  (`/Game/Blueprints/Etc/CharHPBarBP.UpdateLocation` (`self.CharHPBarRef`) (`SceneComponent.K2_GetComponentLocation` (`self.Cube_HPBarPosDummy`)))
  (if (or (`self.isDeathPlayerChar`) (`self.isStageClear`))
    (set `self.CurState` "NewEnumerator3")
    (else
      (switch `/Game/Enums/MonsterState` (`self.CurState`)
        (:`NewEnumerator0`
          (if (<= (`self.DistancePlayerChar`) 500.0)
            (set `self.CurState` "NewEnumerator1")))
        (:`NewEnumerator1`
          (if (>= (`self.DistancePlayerChar`) (`self.AttackRange`))
            (`self.AddMovementInput` (`self.DirToPlayerChar`))
            (else
              (set `self.CurState` "NewEnumerator2"))))
        (:`NewEnumerator2`
          (if (`self.isAttacking`)
            _
            (elif (> (`self.DistancePlayerChar`) (`self.AttackContinueRange`))
              (set `self.CurState` "NewEnumerator1")
              (else
                (`self.Attack`)))))))))

(event `self.ReceiveAnyDamage`
  (params (Damage :type "Float (single-precision)") (DamageType :type "DamageType Object Reference") (InstigatedBy :type "Controller Object Reference") (DamageCauser :type "Actor Object Reference"))
  ;[1 1 1] TakingDamage
  (if (> (`self.TimefromLastDamage`) (`self.DamageDelay`))
    (set `self.TimefromLastDamage` 0.0)
    (if (`|EnumInequality` (`self.CurState`) "NewEnumerator4")
      (bind _output_get (set `self.TakenDamage` Damage))
      (`self.Update HP` _output_get)
      (`/Game/Blueprints/Etc/CharHPBarBP.UpdateHPBar` (`self.CharHPBarRef`) (`self.CurHP`) (`self.MaxHP`))
      (set `self.isDead` (<= (`self.CurHP`) 0.0))
      (`self.Damaged Effect`))))

(event `Update HP`
  (params (TakenDamage :type "Float (double-precision)"))
  ;[1 1 1] TakingDamage
  (set `self.CurHP` (- (`self.CurHP`) TakenDamage)))

(event `self.Capsule.OnComponentBeginOverlap`
  (params (OverlappedComponent :type "PrimitiveComponent Object Reference") (OtherActor :type "Actor Object Reference") (OtherComp :type "PrimitiveComponent Object Reference") (OtherBodyIndex :type Integer) (bFromSweep :type Boolean) (SweepResult :type "HitResult Structure (by ref)"))
  (if (!= OtherActor self)
    (if (== (`|GetArrayItem` (`ActorComponent.ComponentTags` OtherComp)) "Character")
      (if (!= (`|GetArrayItem` (`Actor.Tags` OtherActor)) (`|GetArrayItem` (`self.Tags`)))
        (`GameplayStatics.ApplyDamage` OtherActor (`self.Atk`) null self)))))

(event `Impact Effect`
  ;[1 1 1] TakingDamage
  (`self.PlayAnimMontage` "/Game/Mesh/Goblin/Animations/AnimMontage/goblin_Impact_Montage.goblin_Impact_Montage")
  (set `self.CurState` "NewEnumerator6")
  (`self.LaunchCharacter` (* (* (`self.DirToPlayerChar`) -1.0) 300.0))
  (set `self.isAttacking` false)
  (`PrimitiveComponent.SetCollisionEnabled` (`self.Capsule`) "NoCollision"))

(event `Dying Effect`
  ;[1 1 1] TakingDamage
  (`self.LaunchCharacter` (* (* (`self.DirToPlayerChar`) -1.0) 300.0))
  (`self.PlayAnimMontage` "/Game/Mesh/Goblin/AnimMontage/Goblin_death_Montage.Goblin_death_Montage")
  (set `self.CurState` "NewEnumerator4")
  (`PrimitiveComponent.SetCollisionEnabled` (`self.Capsule`) "NoCollision")
  (`KismetSystemLibrary.Delay` 5.0)
  (`self.K2_DestroyActor`)
  (`self.K2_DestroyActor` (`self.CharHPBarRef`)))

(event `OnCollStart_Attack`
  (`PrimitiveComponent.SetCollisionEnabled` (`self.Capsule`) "QueryOnly"))

(event `CreateDamageText`
  (params (TakenDamage :type "Float (double-precision)"))
  ;[1 1 1] TakingDamage
  (bind _returnvalue (`|SpawnActorFromClass` "/Game/Blueprints/Etc/CharDamageTextBP.CharDamageTextBP_C" (`KismetMathLibrary.MakeTransform` (+ (`SceneComponent.K2_GetComponentLocation` (`self.Cube_DamageTextPosDummy`)) (-60.0 0.0 0.0))) "Undefined" "OverrideRootScale" null null))
  (`/Game/Blueprints/Etc/CharDamageTextBP.SetDamageText` _returnvalue TakenDamage))

(event `Damaged Effect`
  ;[1 1 1] TakingDamage
  (`GameplayStatics.SpawnEmitterAttached` "/Game/InfinityBladeEffects/Effects/FX_Mobile/Fire/combat/P_FireBall_Powerup.P_FireBall_Powerup" (`self.CapsuleComponent`))
  (`self.CreateDamageText` (`self.TakenDamage`))
  (`GameplayStatics.PlaySound2D` "/Game/Sounds/Sword_Stab_Cue.Sword_Stab_Cue" 1.0 1.0 0.0 null null)
  (if (`self.isDead`)
    (`self.Dying Effect`)
    (else
      (`self.Impact Effect`)))
  (`PrimitiveComponent.SetMaterial` (`self.Mesh`) 0 "/Game/Mesh/Goblin/phong1_Inst.phong1_Inst")
  (`KismetSystemLibrary.Delay` 0.2)
  (`PrimitiveComponent.SetMaterial` (`self.Mesh`) 0 "/Game/Mesh/Goblin/phong1.phong1"))

(event `OnCollEnd_Attack`
  (`PrimitiveComponent.SetCollisionEnabled` (`self.Capsule`) "NoCollision"))

(fn `UserConstructionScript`)