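; FollowCamBP is a follow-camera actor that trails player character 0 with smoothed movement.
; On BeginPlay it stores its world-space offset from the character.
; Each tick it lerps its location toward the character's location plus that offset, using delta time times Smooth as alpha, without sweeping.
; It changes only location, so rotation is untouched and the offset does not turn with the character.
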(event `self.ReceiveBeginPlay`
  (set `self.Offset` (- (`self.K2_GetActorLocation`) (`self.K2_GetActorLocation` (`GameplayStatics.GetPlayerCharacter` 0)))))

(event `self.ReceiveTick`
  (params (DeltaSeconds :type "Float (single-precision)"))
  (`self.K2_SetActorLocation` (`KismetMathLibrary.VLerp` (`self.K2_GetActorLocation`) (+ (`self.K2_GetActorLocation` (`GameplayStatics.GetPlayerCharacter` 0)) (`self.Offset`)) (* DeltaSeconds (`self.Smooth`)))))

(fn `UserConstructionScript`)