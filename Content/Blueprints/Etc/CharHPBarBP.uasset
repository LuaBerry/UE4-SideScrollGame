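; CharHPBarBP is an actor that displays a character's health bar through a widget component.
; On BeginPlay it casts the component's widget to CharHPBar and caches its progress bar.
; It exposes UpdateHPBar, which sets the bar to current over max HP, and UpdateLocation, which moves the actor to a given position.
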(event `self.ReceiveBeginPlay`
  (bind _aschar_hpbar (cast `/Game/Blueprints/UI/CharHPBar` (`WidgetComponent.GetUserWidgetObject` (`self.HPBar`))))
  (set `self.HPBar_PBRef` (`/Game/Blueprints/UI/CharHPBar.HPBar` _aschar_hpbar)))

(fn `UpdateHPBar`
  (params (CurHP :type "Float (double-precision)") (MaxHp :type "Float (double-precision)"))
  (`ProgressBar.SetPercent` (`self.HPBar_PBRef`) (/ CurHP MaxHp)))

(fn `UpdateLocation`
  (params (Location :type "Vector Structure"))
  (`self.K2_SetActorLocation` Location))

(fn `UserConstructionScript`)