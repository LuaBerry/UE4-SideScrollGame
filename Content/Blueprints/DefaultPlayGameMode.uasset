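; DefaultPlayGameMode is a game mode that detects when the stage boss reaches a specific state and triggers stage clear.
; On BeginPlay it finds the actor tagged Boss and caches it as a BossMonsterBP.
; Each Tick during the Play state it polls the boss state, then switches to StageClear, shows the StageClear widget, enables the mouse cursor and disables player input.
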(event `self.ReceiveBeginPlay`
  (bind _outactors (`GameplayStatics.GetAllActorsWithTag` "Boss"))
  (bind _asboss_monster_bp (cast `/Game/Blueprints/BossMonsterBP` (`|GetArrayItem` _outactors)))
  (set `self.Boss` _asboss_monster_bp))

(event `self.ReceiveTick`
  (params (DeltaSeconds :type "Float (single-precision)"))
  (bind _returnvalue (`GameplayStatics.GetPlayerController` 0))
  (switch `/Game/Enums/GameplayState` (`self.CurGameplayState`)
    (:`NewEnumerator1`
      (if (`|EnumEquality` (`/Game/Blueprints/BossMonsterBP.CurState` (`self.Boss`)) "NewEnumerator4")
        (set `self.CurGameplayState` "NewEnumerator2")
        (bind _returnvalue_2 (`|CreateWidget` "/Game/Blueprints/UI/StageClear.StageClear_C" _returnvalue))
        (`UserWidget.AddToViewport` _returnvalue_2 0)
        (set `PlayerController.bShowMouseCursor` true _returnvalue)
        (`self.DisableInput` (`GameplayStatics.GetPlayerCharacter` 0) (`GameplayStatics.GetPlayerController` 0))))))

(fn `UserConstructionScript`)