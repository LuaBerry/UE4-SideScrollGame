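; Player character Blueprint with single-axis movement along world Y, a jump and a sword slash, viewed through the Cam view target set at BeginPlay.
; An IsAttacking flag blocks movement input, new attacks and jumps during the slash montage until the OnAnimEnd_Attack event clears it.
; Jumping also requires not falling and plays its own montage, which stops on landing.
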(event `self.ReceiveBeginPlay`
  (`PlayerController.SetViewTargetWithBlend` (`GameplayStatics.GetPlayerController` 0) (`self.Cam`) 0.0 "VTBlend_Linear" 0.0 false))

(event `InputAxis|Left`
  (params (AxisValue :type "Float (single-precision)"))
  (if (not (`self.isAttacking`))
    (`self.AddMovementInput` (0.0 1.0 0.0) AxisValue)))

(event `Key|LeftMouseButton`
  (params (Key :type "Key Structure"))
  (:`Pressed`
    (if (not (`self.isAttacking`))
      (set `self.isAttacking` true)
      (`self.PlayAnimMontage` "/Game/Mesh/Animations/sword_and_shield_slash_Montage.sword_and_shield_slash_Montage"))))

(event `OnAnimEnd_Attack`
  (set `self.isAttacking` false))

(event `Key|SpaceBar`
  (params (Key :type "Key Structure"))
  (:`Pressed`
    (if (`NavMovementComponent.IsFalling` (`self.CharacterMovement`))
      _
      (elif (not (`self.isAttacking`))
        (`self.Jump`)
        (`self.PlayAnimMontage` "/Game/Mesh/Animations/sword_and_shield_jump_Montage.sword_and_shield_jump_Montage"))))
  (:`Released`
    (`self.StopJumping`)))

(event `self.OnLanded`
  (params (Hit :type "HitResult Structure (by ref)"))
  (`self.StopAnimMontage` "/Game/Mesh/Animations/sword_and_shield_jump_Montage.sword_and_shield_jump_Montage"))

(fn `UserConstructionScript`)