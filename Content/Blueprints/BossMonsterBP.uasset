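; Mutant boss for the side-scroller that detects the player, shows the boss HP UI, chases along Y and attacks.
; Tick drives a state machine from player distance, choosing a punch or, once the looping cooldown timer allows, a telegraphed skill swipe.
; Collision events toggle Sphere and Capsule hitboxes, whose tag-filtered overlaps apply damage.
; Incoming damage is rate-limited, updates the HP bar, spawns hit effects, and triggers death and delayed destruction at zero HP.
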(event `self.ReceiveBeginPlay`
  (bind _asside_scroll_game_instance (cast `/Game/Blueprints/SideScrollGameInstance` (`GameplayStatics.GetGameInstance`)))
  (set `self.SideScrollGameInsRef` _asside_scroll_game_instance))

(event `GetDistance_And_Direction`
  (bind _y (.y (- (`self.K2_GetActorLocation` (`GameplayStatics.GetPlayerCharacter` 0)) (`self.K2_GetActorLocation`))))
  (bind _asdefault_play_game_mode (cast `/Game/Blueprints/DefaultPlayGameMode` (`GameplayStatics.GetGameMode`)))
  (set `self.isStageClear` (`|EnumEquality` (`/Game/Blueprints/DefaultPlayGameMode.CurGameplayState` _asdefault_play_game_mode) "NewEnumerator2"))
  (bind _aspaladin_bp (cast `/Game/Blueprints/PaladinBP` (`GameplayStatics.GetPlayerCharacter` 0)))
  (set `self.isDeathPlayerChar` (`/Game/Blueprints/PaladinBP.isDeath` _aspaladin_bp))
  (set `self.DistancePlayerChar` (`KismetMathLibrary.Abs` _y))
  (set `self.DirToPlayerChar` (`KismetMathLibrary.Normal` (`KismetMathLibrary.MakeVector` 0.0 _y))))

(event `self.ReceiveAnyDamage`
  (params (Damage :type "Float (single-precision)") (DamageType :type "DamageType Object Reference") (InstigatedBy :type "Controller Object Reference") (DamageCauser :type "Actor Object Reference"))
  (if (> (`self.TimeFromLastDamage`) (`self.DamageDelay`))
    (set `self.TimeFromLastDamage` 0.0)
    (set `self.TakenDamage` Damage)
    (set `self.CurHP` (- (`self.CurHP`) (`self.TakenDamage`)))
    (`/Game/Blueprints/UI/GamePlayUI.Update_BossHPBar` (`/Game/Blueprints/SideScrollGameInstance.GamePlayUIRef` (`self.SideScrollGameInsRef`)) (`self.CurHP`) (`self.MaxHP`))
    (`self.Damaged Effect`)
    (if (<= (`self.CurHP`) 0.0)
      (`self.PlayAnimMontage` "/Game/Mesh/Boss/AnimMontage/mutant_dying_Montage.mutant_dying_Montage")
      (set `self.CurState` "NewEnumerator4")
      (`PrimitiveComponent.SetCollisionEnabled` (`self.CapsuleComponent`) "NoCollision")
      (`PrimitiveComponent.SetCollisionEnabled` (`self.Capsule`) "NoCollision")
      (`PrimitiveComponent.SetCollisionEnabled` (`self.Sphere`) "NoCollision")
      (`KismetSystemLibrary.Delay` 10.0)
      (`self.K2_DestroyActor`))))

(event `Damaged Effect`
  (`GameplayStatics.SpawnEmitterAttached` "/Game/InfinityBladeEffects/Effects/FX_Mobile/Fire/combat/P_FireBall_Powerup.P_FireBall_Powerup" (`self.CapsuleComponent`))
  (`self.CreateDamageText` (`self.TakenDamage`))
  (`GameplayStatics.PlaySound2D` "/Game/Sounds/Sword_Stab_Cue.Sword_Stab_Cue" 1.0 1.0 0.0 null null)
  (if (`|EnumInequality` (`self.CurState`) "NewEnumerator5")
    (`PrimitiveComponent.SetMaterial` (`self.Mesh`) 0 "/Game/Mesh/Boss/mutant_M_Hit.mutant_M_Hit")
    (`KismetSystemLibrary.Delay` 0.2)
    (`PrimitiveComponent.SetMaterial` (`self.Mesh`) 0 "/Game/Mesh/Boss/mutant_M.mutant_M")))

(event `self.ReceiveTick`
  (params (DeltaSeconds :type "Float (single-precision)"))
  (set `self.TimeFromLastDamage` (+ DeltaSeconds (`self.TimeFromLastDamage`)))
  (`self.GetDistance_And_Direction`)
  (if (`self.isDeathPlayerChar`)
    (set `self.CurState` "NewEnumerator3")
    (else
      (switch `/Game/Enums/MonsterState` (`self.CurState`)
        (:`NewEnumerator0`
          (if (<= (`self.DistancePlayerChar`) (`self.DetectRange`))
            (set `self.CurState` "NewEnumerator1")
            (`/Game/Blueprints/SideScrollGameInstance.ShowBossUI` (`self.SideScrollGameInsRef`) true (`self.BossTexture`))
            (`self.SkillTimeLoop`)))
        (:`NewEnumerator1`
          (if (>= (`self.DistancePlayerChar`) (`self.AttackRange`))
            (`self.AddMovementInput` (`self.DirToPlayerChar`))
            (else
              (set `self.CurState` "NewEnumerator2"))))
        (:`NewEnumerator2`
          (if (`self.isAttacking`)
            _
            (elif (> (`self.DistancePlayerChar`) (`self.AttackContinueRange`))
              (set `self.CurState` "NewEnumerator1")
              (else
                (`self.Attack`)))))))))

(event `OnAnimEnd_Attack`
  (`PrimitiveComponent.SetMaterial` (`self.Mesh`) 0 "/Game/Mesh/Boss/mutant_M.mutant_M")
  (set `self.isAttacking` false)
  (set `self.CurState` "NewEnumerator2"))

(event `CreateDamageText`
  (params (TakenDamage :type "Float (double-precision)"))
  (bind _returnvalue (`|SpawnActorFromClass` "/Game/Blueprints/Etc/CharDamageTextBP.CharDamageTextBP_C" (`KismetMathLibrary.MakeTransform` (+ (`SceneComponent.K2_GetComponentLocation` (`self.Cube_DamageTextPosDummy`)) (-60.0 0.0 0.0))) "Undefined" "OverrideRootScale" null null))
  (`/Game/Blueprints/Etc/CharDamageTextBP.SetDamageText` _returnvalue TakenDamage))

(event `OnCollStart_Attack`
  (`PrimitiveComponent.SetCollisionEnabled` (`self.Sphere`) "QueryOnly"))

(event `SkillTimeLoop`
  (`KismetSystemLibrary.Delay` 1.0)
  (set `self.CurSkillCooledTime` (+ (`self.CurSkillCooledTime`) 1.0))
  (`self.SkillTimeLoop`))

(event `OnCollEnd_Attack`
  (`PrimitiveComponent.SetCollisionEnabled` (`self.Sphere`) "NoCollision"))

(event `OnCollStart_Skill`
  (`PrimitiveComponent.SetCollisionEnabled` (`self.Capsule`) "QueryOnly"))

(event `Attack`
  (set `self.isAttacking` true)
  (if (>= (`self.CurSkillCooledTime`) (`self.SkillCoolTime`))
    (set `self.CurState` "NewEnumerator5")
    (`self.K2_SetActorRotation` (`KismetMathLibrary.Conv_VectorToRotator` (`self.DirToPlayerChar`)))
    (`PrimitiveComponent.SetMaterial` (`self.Mesh`) 0 "/Game/Mesh/Boss/mutant_M_Skill.mutant_M_Skill")
    (`self.PlayAnimMontage` "/Game/Mesh/Boss/AnimMontage/mutant_flexing_muscles_Montage.mutant_flexing_muscles_Montage" 1.0 "Start")
    (`KismetSystemLibrary.Delay` 2.0)
    (if (`|EnumEquality` (`self.CurState`) "NewEnumerator5")
      (`self.PlayAnimMontage` "/Game/Mesh/Boss/AnimMontage/mutant_swiping_Montage.mutant_swiping_Montage")
      (set `self.CurSkillCooledTime` 0.0))
    (else
      (set `self.CurState` "NewEnumerator2")
      (`self.K2_SetActorRotation` (`KismetMathLibrary.Conv_VectorToRotator` (`self.DirToPlayerChar`)))
      (`self.PlayAnimMontage` "/Game/Mesh/Boss/AnimMontage/Mutant_Punch_Montage.Mutant_Punch_Montage"))))

(event `OnCollEnd_Skill`
  (`PrimitiveComponent.SetCollisionEnabled` (`self.Capsule`) "NoCollision"))

(event `self.Sphere.OnComponentBeginOverlap`
  (params (OverlappedComponent :type "PrimitiveComponent Object Reference") (OtherActor :type "Actor Object Reference") (OtherComp :type "PrimitiveComponent Object Reference") (OtherBodyIndex :type Integer) (bFromSweep :type Boolean) (SweepResult :type "HitResult Structure (by ref)"))
  (if (!= OtherActor self)
    (if (== (`|GetArrayItem` (`ActorComponent.ComponentTags` OtherComp)) "Character")
      (if (!= (`|GetArrayItem` (`Actor.Tags` OtherActor)) (`|GetArrayItem` (`self.Tags`)))
        (`GameplayStatics.ApplyDamage` OtherActor (`self.Atk`) null self)))))

(event `self.Capsule.OnComponentBeginOverlap`
  (params (OverlappedComponent :type "PrimitiveComponent Object Reference") (OtherActor :type "Actor Object Reference") (OtherComp :type "PrimitiveComponent Object Reference") (OtherBodyIndex :type Integer) (bFromSweep :type Boolean) (SweepResult :type "HitResult Structure (by ref)"))
  (if (!= OtherActor self)
    (if (== (`|GetArrayItem` (`ActorComponent.ComponentTags` OtherComp)) "Character")
      (if (!= (`|GetArrayItem` (`Actor.Tags` OtherActor)) (`|GetArrayItem` (`self.Tags`)))
        (`GameplayStatics.ApplyDamage` OtherActor (`self.SkillAtk`) null self)))))

(fn `UserConstructionScript`)